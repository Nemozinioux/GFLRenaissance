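; Frag grenade throwable that detonates on a fixed fuse after BeginPlay and damages training dummies in its blast radius.
; A multi-sphere trace gathers candidates, then a line trace to each skips those whose blocking hit is WorldStatic, giving simple cover.
; Remaining TrainingDummy actors receive GrenadeDamage.
; The blast plays a distance-based camera shake and briefly flashes a point light before the actor destroys itself.
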(event EventBeginPlay
  (bind _returnvalue (Transformation|GetActorLocation))
  (Utilities|FlowControl|Delay 3.5)
  (bind _outhits (Collision|MultiSphereTraceByChannel _returnvalue _returnvalue 5e+02 "TraceTypeQuery1" false 0 "None"))
  (for _array_element _outhits
    (bind _outhit (Collision|LineTraceByChannel (Transformation|GetActorLocation) (Transformation|GetActorLocation (.HitActor (Collision|BreakHitResult _array_element))) "TraceTypeQuery1" false 0 "None"))
    (Utilities|IsValid (.hitcomponent _outhit)
      (:Is%20Valid
        (if (not (Utilities|Enum|Equal(Enum) (Utilities|String|EnumtoString (Collision|GetCollisionObjectType (.hitcomponent _outhit))) "WorldStatic"))
          (bind _astraining_dummy (Utilities|Casting|CastToTrainingDummy (.HitActor (Collision|BreakHitResult _array_element))))
          (Default|GrenadeDamage _astraining_dummy)))))
  (Camera|PlayWorldCameraShake "/Game/PlayerCharacter/CameraManagement/ScreenShakes/ExplosionShake.ExplosionShake_C" (Transformation|GetActorLocation) 1e+02 1.8e+03)
  (Rendering|SetVisibility (Variables|Default|GetPointLight) true false)
  (Utilities|FlowControl|Delay 0.1)
  (Actor|DestroyActor))

(fn ConstructionScript)